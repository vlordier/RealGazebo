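; BP_LC62Pawn is an aerial vehicle pawn for the LC62 aircraft, with eight propellers and five control surfaces.
; On BeginPlay it fills the RotatingComponents array and binds each rotation movement component to its own propeller through SetUpdatedComponent.
; It then fills ControllableComponents with the left and right ailerons, left and right elevators, and rudder.
; The graphs only register these parts and contain no flight or input logic.
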(event EventBeginPlay
  (Variables|Default|SetRotatingComponents (Utilities|Array|MakeArray (Variables|RealGazebo|GetRotation0) (Variables|RealGazebo|GetRotation1) (Variables|RealGazebo|GetRotation2) (Variables|RealGazebo|GetRotation3) (Variables|RealGazebo|GetRotation4) (Variables|RealGazebo|GetRotation5) (Variables|RealGazebo|GetRotation6) (Variables|RealGazebo|GetRotation7)))
  (CallFunction|SetupPropRotationMovement)
  (Variables|Default|SetControllableComponents (Utilities|Array|MakeArray (Variables|Default|GetLeftAil) (Variables|Default|GetRightAil) (Variables|Default|GetLeftEle) (Variables|Default|GetRightEle) (Variables|Default|GetRudder))))

(fn ConstructionScript)

(fn SetupPropRotationMovement
  (Components|Movement|SetUpdatedComponent (Variables|RealGazebo|GetRotation0) (Variables|Default|GetProp0))
  (Components|Movement|SetUpdatedComponent (Variables|RealGazebo|GetRotation1) (Variables|Default|GetProp1))
  (Components|Movement|SetUpdatedComponent (Variables|RealGazebo|GetRotation2) (Variables|Default|GetProp2))
  (Components|Movement|SetUpdatedComponent (Variables|RealGazebo|GetRotation3) (Variables|Default|GetProp3))
  (Components|Movement|SetUpdatedComponent (Variables|RealGazebo|GetRotation4) (Variables|Default|GetProp4))
  (Components|Movement|SetUpdatedComponent (Variables|RealGazebo|GetRotation5) (Variables|Default|GetProp5))
  (Components|Movement|SetUpdatedComponent (Variables|RealGazebo|GetRotation6) (Variables|Default|GetProp6))
  (Components|Movement|SetUpdatedComponent (Variables|RealGazebo|GetRotation7) (Variables|Default|GetProp7))
  (return))